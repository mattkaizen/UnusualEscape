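; BP_Playerz is the player Blueprint, moving on the XY plane through Enhanced Input, with IMC_Player registered at BeginPlay.
; IA_Move offsets the location by ScaleMovement, line-traces at fixed height with persistent debug drawing, and teleports unless it hits a PaperTileMapComponent.
; Successful moves record Directionality, while press and release toggle IsHoldingMove.
; The construction script caches the level's PaperTileMapActor; an AddMovementInput path remains disconnected.
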(event Input|EnhancedActionEvents|EnhancedInputActionIA_Move
  (params (ActionValue :type Vector%202D%20Structure) (ElapsedSeconds :type Float%20%28double-precision%29) (TriggeredSeconds :type Float%20%28double-precision%29) (InputAction :type Input%20Action%20Object%20Reference :default "/Game/Blueprints/Player/Input/IA_Move.IA_Move"))
  (bind _returnvalue (Transformation|GetActorLocation))
  (bind _returnvalue_2 (Transformation|GetActorLocation))
  (:Triggered
    (bind _output_get (Variables|Default|SettargetLocation (Math|Vector|MakeVector (+ (* (Variables|Default|GetscaleMovement) (.x ActionValue)) (.x _returnvalue_2)) (+ (.y _returnvalue_2) (* (Variables|Default|GetscaleMovement) (.y ActionValue))) (.z _returnvalue_2))))
    (bind _outhit (Collision|LineTraceByChannel (Math|Vector|MakeVector (.x _returnvalue) (.y _returnvalue) 5e+01) (Math|Vector|MakeVector (.x _output_get) (.y _output_get) 5e+01) "TraceTypeQuery1" false 0 "Persistent"))
    (Utilities|Casting|CastToPaperTileMapComponent (.HitComponent (Collision|BreakHitResult _outhit))
      (:CastFailed
        (Transformation|SetActorLocation (Variables|Default|GettargetLocation) false false)
        (Variables|Default|Setdirectionality (Math|Vector2D|MakeVector2D (.x ActionValue) (.y ActionValue))))))
  (:Started
    (Variables|Default|SetisHoldingMove? true)))

(event Input|EnhancedActionEvents|EnhancedInputActionIA_Move
  (params (ActionValue :type Vector%202D%20Structure) (ElapsedSeconds :type Float%20%28double-precision%29) (TriggeredSeconds :type Float%20%28double-precision%29) (InputAction :type Input%20Action%20Object%20Reference :default "/Game/Blueprints/Player/Input/IA_Move.IA_Move"))
  (:Started
    (Variables|Default|SetisHoldingMove? true))
  (:Completed
    (Variables|Default|SetisHoldingMove? false)))

(event EventBeginPlay
  (bind _asplayer_controller (Utilities|Casting|CastToPlayerController (Pawn|GetController)))
  (Input|AddMappingContext (PlayerController|LocalPlayerSubsystems|GetEnhancedInputLocalPlayerSubsystem _asplayer_controller) "/Game/Blueprints/Player/Input/IMC_Player.IMC_Player" 0 "(bIgnoreAllPressedKeysUntilRelease=True,bForceImmediately=False)"))

(fn ConstructionScript
  (bind _returnvalue (Actor|GetActorOfClass "/Script/Paper2D.PaperTileMapActor"))
  (Variables|Default|SettileMap _returnvalue))