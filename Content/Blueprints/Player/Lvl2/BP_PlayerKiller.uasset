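; Level 2 player killer actor that kills the player when a BP_SetTile reports them over a dangerous tile.
; The construction script caches every BP_SetTile, and BeginPlay finds BP_Playerz and binds KillPlayer to each tile's OnPlayerOveringDangerousTile event.
; KillPlayer hides the player sprite, clears IsAlive and calls OnPlayerKilled to announce the death.
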(event Custom|KillPlayer
  (Rendering|SetVisibility (Variables|/Script/Paper2D.PaperCharacter|GetSprite (Variables|Default|GetPlayerCharacter)) false false)
  (Variables|/Game/Blueprints/Player/BP_Playerz.BP_Playerz_C|SetisAlive (stale EventBeginPlay _returnvalue) false)
  (Default|CallOnPlayerKilled))

(event EventBeginPlay
  (bind _returnvalue (Actor|GetActorOfClass "/Game/Blueprints/Player/BP_Playerz.BP_Playerz_C"))
  (Variables|Default|SetPlayerCharacter _returnvalue)
  (for _array_element (Variables|Default|GetBP%20SetTile)
    (EventDispatchers|BindEventtoOnPlayerOveringDangerousTile _array_element (delegate Custom|KillPlayer))))

(fn ConstructionScript
  (bind _outactors (Actor|GetAllActorsOfClass "/Game/Blueprints/Tiles/BP_SetTile.BP_SetTile_C"))
  (Variables|Default|SetBP%20SetTile _outactors))