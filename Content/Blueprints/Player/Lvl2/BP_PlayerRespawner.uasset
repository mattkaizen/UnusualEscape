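; BP_PlayerRespawner sends the player back to a PlayerStart when a dangerous tile reports the player over it.
; Its construction script stores a single BP_SetTile, found with GetActorOfClass, in the BPSetTile array.
; BeginPlay caches BP_Playerz and binds KillPlayer to each stored tile's dangerous-tile event.
; KillPlayer teleports the player to the start location with zero rotation and prints that location.
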(event Custom|KillPlayer
  (bind _player_start (Variables|Default|GetPlayer%20Start))
  (bind _returnvalue (Transformation|GetActorLocation _player_start))
  (Transformation|Teleport (Variables|Default|GetPlayerCharacter) _returnvalue "0, 0, 0")
  (Development|PrintString (Utilities|String|ToString(Integer) _returnvalue)))

(event EventBeginPlay
  (bind _returnvalue (Actor|GetActorOfClass "/Game/Blueprints/Player/BP_Playerz.BP_Playerz_C"))
  (Variables|Default|SetPlayerCharacter _returnvalue)
  (for _array_element (Variables|Default|GetBP%20SetTile)
    (EventDispatchers|BindEventtoOnPlayerOveringDangerousTile _array_element (delegate Custom|KillPlayer))))

(fn ConstructionScript
  (bind _returnvalue (Actor|GetActorOfClass "/Game/Blueprints/Tiles/BP_SetTile.BP_SetTile_C"))
  (Variables|Default|SetBP%20SetTile (Utilities|Array|MakeArray _returnvalue)))