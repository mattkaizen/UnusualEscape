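; BP_PlayerRespawn respawns the level's player character after it is killed.
; On BeginPlay it caches the BP_Playerz actor and binds to the OnPlayerKilled event of BP_PlayerKiller.
; When that fires, it waits RespawnTime, teleports the player to PlayerStart, restores sprite visibility and the IsAlive flag, then calls the PlayerRespawned dispatcher.
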(event Custom|PlayerRespawn
  (Utilities|FlowControl|Delay (Variables|Default|GetRespawn%20Time))
  (CallFunction|TeleportPlayer)
  (Rendering|SetVisibility (Variables|/Script/Paper2D.PaperCharacter|GetSprite (Variables|Default|GetPlayer%20Character)) true false)
  (Variables|/Game/Blueprints/Player/BP_Playerz.BP_Playerz_C|SetisAlive (stale EventBeginPlay _returnvalue) true)
  (Default|CallPlayerRespawned))

(event EventBeginPlay
  (bind _returnvalue (Actor|GetActorOfClass "/Game/Blueprints/Player/BP_Playerz.BP_Playerz_C"))
  (Variables|Default|SetPlayer%20Character _returnvalue)
  (bind _returnvalue_2 (Actor|GetActorOfClass "/Game/Blueprints/Player/Lvl2/BP_PlayerKiller.BP_PlayerKiller_C"))
  (EventDispatchers|BindEventtoOnPlayerKilled _returnvalue_2 (delegate Custom|PlayerRespawn)))

(fn ConstructionScript)

(fn TeleportPlayer
  (Transformation|Teleport (Variables|Default|GetPlayer%20Character) (Transformation|GetActorLocation (Variables|Default|GetPlayer%20Start)) "0, 0, 0"))