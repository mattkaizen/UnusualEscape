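; BP_PlayerAudio plays 2D sound effects for player movement, death and respawn.
; On BeginPlay it finds BP_Playerz, BP_PlayerRespawn and BP_PlayerKiller with GetActorOfClass and binds handlers to their move, respawn and killed dispatchers.
; Each handler plays its sound, with the move sound played quietly at a random pitch for variation and the kill event using the fall sound.
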(event Custom|PlayerKilled
  (Audio|PlaySound2D (Variables|Default|GetFallSound) 1.0 1.0 0.0 0 0))

(event Custom|PlayerRespawned
  (Audio|PlaySound2D (Variables|Default|GetRespawnSound) 1.0 1.0 0.0 0 0))

(event Custom|PlayerMove
  (Audio|PlaySound2D (Variables|Default|GetmoveSound) 0.1 (Math|Random|RandomFloatinRange 0.8 1.2) 0.0 0 0))

(event EventBeginPlay
  (bind _returnvalue (Actor|GetActorOfClass "/Game/Blueprints/Player/BP_Playerz.BP_Playerz_C"))
  (EventDispatchers|BindEventtoOnPlayerMove _returnvalue (delegate Custom|PlayerMove))
  (bind _returnvalue_2 (Actor|GetActorOfClass "/Game/Blueprints/Player/Lvl2/BP_PlayerRespawn.BP_PlayerRespawn_C"))
  (EventDispatchers|BindEventtoPlayerRespawned _returnvalue_2 (delegate Custom|PlayerRespawned))
  (bind _returnvalue_3 (Actor|GetActorOfClass "/Game/Blueprints/Player/Lvl2/BP_PlayerKiller.BP_PlayerKiller_C"))
  (EventDispatchers|BindEventtoOnPlayerKilled _returnvalue_3 (delegate Custom|PlayerKilled)))

(fn ConstructionScript)