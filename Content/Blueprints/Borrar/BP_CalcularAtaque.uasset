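; BP_CalcularAtaque is a Blueprint that computes attack damage and prints the results on screen.
; On BeginPlay it runs CalcularAtaqueSimple on PoderBase, a fixed linear formula, then after a delay prints a colored Spanish effectiveness message based on a damage threshold.
; CalcularAtaqueComplejo adds a buff multiplier, random extra damage and enemy armor subtraction, but the event graph never calls it.
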(event EventBeginPlay
  (bind _infligeddamage (CallFunction|CalcularAtaqueSimple (Variables|Default|GetPoder%20Base)))
  (Utilities|FlowControl|Delay 2.0)
  (if (>= _infligeddamage 40)
    (Development|PrintString "Es super Efectivo" true true "(R=0.474190,G=1.000000,B=0.506528,A=1.000000)")
    (else
      (Development|PrintString "No tiene efecto" true true "(R=1.000000,G=0.812949,B=0.167383,A=1.000000)"))))

(event Collision|EventActorBeginOverlap
  (params (OtherActor :type Actor%20Object%20Reference)))

(event EventTick
  (params (DeltaSeconds :type Float%20%28single-precision%29)))

(fn ConstructionScript)

(fn CalcularAtaqueSimple
  (params (Base :type Integer))
  (bind _returnvalue (* Base 5))
  (bind _returnvalue_2 (+ _returnvalue 10))
  (Development|PrintString (Utilities|String|Append "Damage: " (Utilities|String|ToString(Integer) _returnvalue_2)))
  (return _returnvalue_2))

(fn CalcularAtaqueComplejo
  (params (Base :type Integer))
  (bind _buff (Variables|Default|GetBuff))
  (bind _extra_damage (Variables|Default|GetExtra%20Damage))
  (bind _enemy_armor (Variables|Default|GetEnemy%20Armor))
  (bind _returnvalue (Math|Random|RandomIntegerinRange 0 _extra_damage))
  (bind _returnvalue_2 (* Base _buff))
  (bind _returnvalue_3 (+ _returnvalue_2 _returnvalue))
  (bind _returnvalue_4 (- _returnvalue_3 _enemy_armor))
  (Development|PrintString (Utilities|String|Append "Damage: " (Utilities|String|ToString(Integer) _returnvalue_4)))
  (return _returnvalue_4))