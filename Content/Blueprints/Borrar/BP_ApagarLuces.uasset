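; BP_ApagarLuces is a trigger actor that toggles point light visibility when a Character overlaps it.
; An optional flag fills its light array with every PointLight actor in the level.
; Sequential mode toggles only the light at the counter index, then resets the counter to zero without ever advancing it.
; Otherwise it toggles every light in the array, so repeated overlaps switch them back.
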(event Collision|EventActorBeginOverlap
  (params (OtherActor :type Actor%20Object%20Reference))
  (Utilities|Casting|CastToCharacter OtherActor)
  (if (Variables|Default|GetObtener%20Todas%20Las%20Luces)
    (bind _outactors (Actor|GetAllActorsOfClass "/Script/Engine.PointLight"))
    (Variables|Default|SetArrayLuces _outactors))
  (if (Variables|Default|GetSecuencial%20?)
    (Development|PrintString (Utilities|String|ToString(Integer) (Variables|Default|GetContador)))
    (Rendering|ToggleVisibility (Variables|/Script/Engine.PointLight|GetPointLightComponent (Utilities|Array|Get(acopy) (Variables|Default|GetArrayLuces) (Variables|Default|GetContador))) false)
    (Variables|Default|SetContador 0)
    (else
      (for _array_element (Variables|Default|GetArrayLuces)
        (Rendering|ToggleVisibility (Variables|/Script/Engine.PointLight|GetPointLightComponent _array_element) true)))))

(fn ConstructionScript)