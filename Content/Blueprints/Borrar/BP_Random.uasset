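; Debug Blueprint that tries out randomness and flow-control nodes through number-key presses.
; Key 9 rolls two random integers from 0 to 6 as dice and prints both with their sum.
; Key 8 uses a looping random MultiGate to swap a StaticMeshActor's material among three instances.
; Releasing 8 prints Hello through a DoN limited to five times, which key 7 resets.
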(event Input|KeyboardEvents|9
  (params (Key :type Key%20Structure :default "None"))
  (:Pressed
    (Variables|Default|SetDado%201 (Math|Random|RandomIntegerinRange 0 6))
    (Variables|Default|SetDado%202 (Math|Random|RandomIntegerinRange 0 6))
    (Development|PrintString (Utilities|String|Append "Dado 1: " (Utilities|String|ToString(Integer) (Variables|Default|GetDado%201)) " Dado 2 " (Utilities|String|ToString(Integer) (Variables|Default|GetDado%202)) " Suma: " (Utilities|String|ToString(Integer) (+ (Variables|Default|GetDado%201) (Variables|Default|GetDado%202))) " FIN"))))

(event Input|KeyboardEvents|8
  (params (Key :type Key%20Structure :default "None"))
  (bind _static_mesh_actor (Variables|Default|GetStatic%20Mesh%20Actor))
  (bind _staticmeshcomponent (Variables|/Script/Engine.StaticMeshActor|GetStaticMeshComponent _static_mesh_actor))
  (:Pressed
    ;[0.1572 0.02821 0.2708] Control de flujo
    (Utilities|FlowControl|MultiGate true true -1
      (:Out%200
        (Rendering|Material|SetMaterial _staticmeshcomponent 0 "/Game/Materials/M_Noise_Inst.M_Noise_Inst"))
      (:Out%201
        (Rendering|Material|SetMaterial _staticmeshcomponent 0 "/Game/Materials/M_Gold_Inst.M_Gold_Inst"))
      (:Out%202
        (Rendering|Material|SetMaterial _staticmeshcomponent 0 "/Game/Materials/M_Power_Inst.M_Power_Inst"))))
  (:Released
    (Utilities|FlowControl|DoN 5
      (:Exit
        (Development|PrintString "Hello")))))

(event Input|KeyboardEvents|7
  (params (Key :type Key%20Structure :default "None"))
  (:Pressed
    (Utilities|FlowControl|DoN 5) ; enters at Reset
  ))

(fn ConstructionScript)