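; BP_SetTile is a trigger actor that swaps one dungeon tilemap tile when a Character overlaps it, with a crack sound.
; Each Character overlap calls the OnPlayerOveringDangerousTile dispatcher.
; A DoOnce then limits the change to the first overlap, setting the tile at the configured coordinates and layer on TMDungeon to a new TS_Dungeon tile and playing the sound.
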(event Collision|EventActorBeginOverlap
  (params (OtherActor :type Actor%20Object%20Reference))
  (Utilities|Casting|CastToCharacter OtherActor)
  (Default|CallOnPlayerOveringDangerousTile)
  (Utilities|FlowControl|DoOnce false
    (:Completed
      (Class|PaperTileMapComponent|SetTile (Variables|/Script/Paper2D.PaperTileMapActor|GetRenderComponent (Variables|Default|GetTM_Dungeon)) (Variables|Default|GetTile%20Index%20X%20To%20Modify) (Variables|Default|GetTile%20Index%20Y%20To%20Modify) (Variables|Default|GetTM%20Layer) (Utilities|Struct|MakePaperTileInfo (Variables|Default|GetNew%20Tile%20Index) "/Game/Assets/Textures/Tiles/TS_Dungeon.TS_Dungeon" false false false))
      (Audio|PlaySound2D "/Game/Assets/Audio/Tile/tileCrackSound2.tileCrackSound2" 1.0 1.0 0.0 0 0))))

(fn ConstructionScript)